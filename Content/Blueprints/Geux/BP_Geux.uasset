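; BP_Geux is an actor that shows a random image from the AllGeux set on a widget and animates it vertically in a continuous loop.
; On BeginPlay it sets the WB_Geux image and waits a random delay, so instances start out of sync.
; The TL_Geux timeline lerps the actor between its start location and a point above, restarting on finish with a new random play rate each cycle.
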(event `self.ReceiveBeginPlay`
  (bind _returnvalue (`self.K2_GetActorLocation` self))
  (set `self.Texture` (`KismetArrayLibrary.Array_Random` (`self.AllGeux`)))
  (`Image.SetBrushFromTexture` (`/Game/Blueprints/Geux/WB_Geux.Image` (cast `/Game/Blueprints/Geux/WB_Geux` (`WidgetComponent.GetWidget` (`self.Widget`)) :!pure true)) (`self.Texture`) false)
  (set `self.StartLoc` _returnvalue)
  (set `self.EndLoc` (+ _returnvalue (0.0 0.0 250.0)))
  (`KismetSystemLibrary.Delay` (`KismetMathLibrary.RandomFloatInRange` 0.0 3.0))
  (`self.StartLoop`))

(event `StartLoop`
  (`TimelineComponent.SetPlayRate` (`self.TL_Geux`) (/ 1.0 (`KismetMathLibrary.RandomFloatInRange` 0.35 0.75)))
  (bind (_direction _alpha) (`Timeline|TL_Geux` :!via `PlayFromStart`)
    (:`Update`
      (`self.K2_SetActorLocation` (`KismetMathLibrary.VLerp` (`self.StartLoc`) (`self.EndLoc`) _alpha)))
    (:`Finished`
      (`self.StartLoop`))))

(fn `UserConstructionScript`)