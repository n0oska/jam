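; BP_Bullet3 is a physics-driven bullet that damages enemies.
; On BeginPlay it finds BP_Character and launches its Sphere with a strong impulse along the forward vector of that character's SpawnBulletRefDistance.
; Sphere1 overlaps with BP_EnnemiParent actors call TakedamageE with a random roll whose equal bounds make it fixed, and print the value.
; The graph never destroys the bullet.
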(event `self.ReceiveBeginPlay`
  (bind _returnvalue (`GameplayStatics.GetActorOfClass` "/Game/Blueprints/Character/BP_Character.BP_Character_C"))
  (set `self.Player` _returnvalue)
  (`PrimitiveComponent.AddImpulse` (`self.Sphere`) (* (`SceneComponent.GetForwardVector` (`/Game/Blueprints/Character/BP_Character.SpawnBulletRefDistance` _returnvalue)) 15000.0) "None" false))

(event `self.Sphere1.OnComponentBeginOverlap`
  (params (OverlappedComponent :type "PrimitiveComponent Object Reference") (OtherActor :type "Actor Object Reference") (OtherComp :type "PrimitiveComponent Object Reference") (OtherBodyIndex :type Integer) (bFromSweep :type Boolean) (SweepResult :type "HitResult Structure (by ref)"))
  (bind _returnvalue (`KismetMathLibrary.RandomIntegerInRange` 50 50))
  (bind (_asbp_ennemi_parent _bsuccess) (cast `/Game/Blueprints/Ennemi/BP_EnnemiParent` OtherActor :!pure true))
  (if _bsuccess
    (`/Game/Blueprints/Ennemi/BP_EnnemiParent.takedamageE` _asbp_ennemi_parent (`KismetMathLibrary.Conv_IntToDouble` _returnvalue))
    (`KismetSystemLibrary.PrintString` (`KismetStringLibrary.Conv_IntToString` _returnvalue))))

(fn `UserConstructionScript`)