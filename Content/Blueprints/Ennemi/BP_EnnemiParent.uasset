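; Parent enemy that chases and attacks the player as one of three EnnemiType variants, each with its own mesh and stats.
; Looping timers drive AIMoveTo chases; timelines animate facing and attacks.
; Sphere overlap triggers Basic's lunge or Braum's slam, while Distance throws within range along a GameManager spline arc.
; Attacks damage the player on completion without gating on a hit; Braum blocks Bullet3-tagged actors, and death updates the score combo.
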(event `OnSwitch`
  (switch `/Game/Blueprints/Ennemi/E_EnnemiType` (`self.EnnemiType`) :!label _label
    (:`NewEnumerator0`
      (`self.BaseEnnemi_StartPatrol`))
    (:`NewEnumerator1`
      (`self.BraumSetup`))
    (:`NewEnumerator2`
      (`self.DistanceSetup`))))

(event `self.ReceiveBeginPlay`
  (bind _returnvalue (`GameplayStatics.GetActorOfClass` "/Game/Blueprints/Character/BP_Character.BP_Character_C"))
  (set `self.Player` _returnvalue)
  (bind _returnvalue_2 (`GameplayStatics.GetActorOfClass` "/Game/Blueprints/Manager/BP_GameManager.BP_GameManager_C"))
  (set `self.GameManager` _returnvalue_2)
  (`KismetSystemLibrary.DelayUntilNextTick`)
  (goto _label))

(event `self.Sphere.OnComponentBeginOverlap`
  (params (OverlappedComponent :type "PrimitiveComponent Object Reference") (OtherActor :type "Actor Object Reference") (OtherComp :type "PrimitiveComponent Object Reference") (OtherBodyIndex :type Integer) (bFromSweep :type Boolean) (SweepResult :type "HitResult Structure (by ref)"))
  (if (`.bSuccess` (cast `/Game/Blueprints/Character/BP_Character` OtherActor :!pure true))
    (switch `/Game/Blueprints/Ennemi/E_EnnemiType` (`self.EnnemiType`)
      (:`NewEnumerator0`
        (`self.BaseAttack`))
      (:`NewEnumerator1`
        (`self.BraumAttack`)))))

(event `self.Sphere.OnComponentEndOverlap`
  (params (OverlappedComponent :type "PrimitiveComponent Object Reference") (OtherActor :type "Actor Object Reference") (OtherComp :type "PrimitiveComponent Object Reference") (OtherBodyIndex :type Integer))
  (if (`.bSuccess` (cast `/Game/Blueprints/Character/BP_Character` OtherActor :!pure true))
    (switch `/Game/Blueprints/Ennemi/E_EnnemiType` (`self.EnnemiType`)
      (:`NewEnumerator0`
        (set `self.bCanAttackPlayer` false))
      (:`NewEnumerator1`
        (set `self.bCanAttackPlayerBraum` false)))))

(event `BaseEnnemi_StartPatrol`
  ;[1 0 0 0.1] Base Ennemi
  (bind _returnvalue (`KismetSystemLibrary.K2_SetTimerDelegate` (delegate `Code`) 0.25 true))
  (set `self.Handle_Patrol` _returnvalue)
  (bind _output_get (set `self.MaxHealth` 100.0))
  (set `self.CurrentHealth` _output_get)
  (set `CharacterMovementComponent.MaxWalkSpeed` 800.0 (`self.CharacterMovement`))
  (`SkeletalMeshComponent.SetSkeletalMeshAsset` (`self.Mesh`) "/Game/Blueprints/Ennemi/mesh/Chien/SKM_JAM_Chien_fix.SKM_JAM_Chien_fix"))

(event `Code`
  (bind (_returnvalue_roll _returnvalue_pitch _returnvalue_yaw) (`KismetMathLibrary.BreakRotator` (`KismetMathLibrary.FindLookAtRotation` (`self.K2_GetActorLocation` self) (`self.K2_GetActorLocation` (`self.Player`)))))
  (bind _returnvalue (+ _returnvalue_yaw 270.0))
  ;[1 0 0 0.1] Base Ennemi
  (`|AIMoveTo` self (0.0 0.0 0.0) (`self.Player`)
    (:`then`
      (`TimelineComponent.SetPlayRate` (`self.TL_MovementEnnemi`) (/ 1.0 0.24))
      (`Timeline|TL_MovementEnnemi` :!via `PlayFromStart`
        (:`Update`
          (set `self.forward` (`KismetMathLibrary.Conv_DoubleToVector` _returnvalue))
          (`self.K2_SetActorRotation` self (`KismetMathLibrary.MakeRotator` 0.0 0.0 _returnvalue) false))))))

(event `BaseAttack`
  (bind _player (`self.Player`))
  ;[1 0 0 0.1] Base Ennemi
  (set `self.bCanAttackPlayer` true)
  (`KismetSystemLibrary.Delay` 0.5)
  (if (`self.bCanAttackPlayer`)
    (`KismetSystemLibrary.K2_ClearAndInvalidateTimerHandle` (`self.Handle_Patrol`))
    (`MovementComponent.StopMovementImmediately` (`self.CharacterMovement`))
    (`TimelineComponent.SetPlayRate` (`self.TL_AttackPlayer`) (/ 1.0 2.0))
    (bind (_direction _alpha _alphalocation) (`Timeline|TL_AttackPlayer` :!via `PlayFromStart`)
      (:`Update`
        (if (< _alpha 0.5)
          (bind (_returnvalue_roll _returnvalue_pitch _returnvalue_yaw) (`KismetMathLibrary.BreakRotator` (`KismetMathLibrary.RLerp` (`self.K2_GetActorRotation` self) (`KismetMathLibrary.FindLookAtRotation` (`self.K2_GetActorLocation` self) (`self.K2_GetActorLocation` (`self.Player`))) _alpha true)))
          (`self.K2_SetActorRotation` self (`KismetMathLibrary.MakeRotator` 0.0 0.0 (+ _returnvalue_yaw 270.0)) false)
          (else
            (`|ExecutionSequence`
              (:`then_0`
                (`/Engine/EditorBlueprintResources/StandardMacros.DoOnce` false :!label _label_2
                  (:`Completed`
                    (set `self.AttackPlayerLocation` (`self.K2_GetActorLocation` (`self.Player`))))))
              (:`then_1`
                (`self.K2_SetActorLocation` self (`KismetMathLibrary.VLerp` (`self.K2_GetActorLocation` self) (`self.AttackPlayerLocation`) _alphalocation) false false))))))
      (:`Finished`
        (`TimelineComponent.SetPlayRate` (`self.TL_GoBackToPlayer`) (/ 1.0 0.3))
        (bind (_direction_2 _alpha_2) (`Timeline|TL_GoBackToPlayer` :!via `PlayFromStart`)
          (:`Update`
            (bind (_returnvalue_roll_2 _returnvalue_pitch_2 _returnvalue_yaw_2) (`KismetMathLibrary.BreakRotator` (`KismetMathLibrary.RLerp` (`self.K2_GetActorRotation` self) (`KismetMathLibrary.FindLookAtRotation` (`self.K2_GetActorLocation` self) (`self.K2_GetActorLocation` (`self.Player`))) _alpha_2 true)))
            (`self.K2_SetActorRotation` self (`KismetMathLibrary.MakeRotator` 0.0 0.0 (+ _returnvalue_yaw_2 280.0)) false))
          (:`Finished`
            (`self.BaseEnnemi_StartPatrol`)
            (`self.ResetDoOnce`)
            (`/Game/Blueprints/Character/BP_Character.takedamage` _player (`KismetMathLibrary.Conv_IntToDouble` (`KismetMathLibrary.RandomIntegerInRange` 5 7)))
            (`KismetSystemLibrary.PrintString` (`KismetStringLibrary.Conv_DoubleToString` (`/Game/Blueprints/Character/BP_Character.current health` _player)))))))))

(event `ResetDoOnce`
  ;[1 0 0 0.1] Base Ennemi
  (goto _label_2 :!via `Reset`))

(event `BraumSetup`
  ;[0 1 0 0.1] Braum
  (`SceneComponent.SetWorldScale3D` (`self.Sphere`) (`self.ScaleAttackDetectionBraum`))
  (bind _output_get (set `self.MaxHealth` 150.0))
  (set `self.CurrentHealth` _output_get)
  (set `CharacterMovementComponent.MaxWalkSpeed` 600.0 (`self.CharacterMovement`))
  (`SkeletalMeshComponent.SetSkeletalMeshAsset` (`self.Mesh`) "/Game/Blueprints/Ennemi/mesh/Renneù/SKM_JAM_Rennes_fix.SKM_JAM_Rennes_fix")
  (`self.Braum_StartPatrol`))

(event `self.Box.OnComponentBeginOverlap`
  (params (OverlappedComponent :type "PrimitiveComponent Object Reference") (OtherActor :type "Actor Object Reference") (OtherComp :type "PrimitiveComponent Object Reference") (OtherBodyIndex :type Integer) (bFromSweep :type Boolean) (SweepResult :type "HitResult Structure (by ref)"))
  ;[0 1 0 0.1] Braum
  (if (and (`self.ActorHasTag` OtherActor "Bullet3") (`|EnumEquality` (`self.EnnemiType`) "NewEnumerator1"))
    (`self.K2_DestroyActor` OtherActor)))

(event `Braum_StartPatrol`
  ;[0 1 0 0.1] Braum
  (bind _returnvalue (`KismetSystemLibrary.K2_SetTimerDelegate` (delegate `CodeBraum`) 0.25 true))
  (set `self.Handle_Patrol_Braum` _returnvalue))

(event `CodeBraum`
  (bind (_returnvalue_roll _returnvalue_pitch _returnvalue_yaw) (`KismetMathLibrary.BreakRotator` (`KismetMathLibrary.FindLookAtRotation` (`self.K2_GetActorLocation` self) (`self.K2_GetActorLocation` (`self.Player`)))))
  ;[0 1 0 0.1] Braum
  (`|AIMoveTo` self (0.0 0.0 0.0) (`self.Player`)
    (:`then`
      (`TimelineComponent.SetPlayRate` (`self.TL_PatrolBraum`) (/ 1.0 0.24))
      (`Timeline|TL_PatrolBraum` :!via `PlayFromStart`
        (:`Update`
          (`self.K2_SetActorRotation` self (`KismetMathLibrary.MakeRotator` 0.0 0.0 (+ _returnvalue_yaw 280.0)) false))))))

(event `BraumAttack`
  (bind _returnvalue (`self.K2_GetActorLocation` self))
  ;[0 1 0 0.1] Braum
  (`KismetSystemLibrary.K2_ClearAndInvalidateTimerHandle` (`self.Handle_Patrol_Braum`))
  (`MovementComponent.StopMovementImmediately` (`self.CharacterMovement`))
  (set `self.StartLocAttackBraum` _returnvalue)
  (set `self.EndLocAttackBraum` (+ _returnvalue (0.0 0.0 150.0)))
  (`TimelineComponent.SetPlayRate` (`self.TL_AttackBraum`) (/ 1.0 0.75))
  (set `CharacterMovementComponent.GravityScale` 0.0 (`self.CharacterMovement`))
  (bind (_direction _alpha) (`Timeline|TL_AttackBraum` :!via `PlayFromStart`)
    (:`Update`
      (`self.K2_SetActorLocation` self (`KismetMathLibrary.VLerp` (`self.StartLocAttackBraum`) (`self.EndLocAttackBraum`) _alpha) false false))
    (:`Finished`
      (`TimelineComponent.SetPlayRate` (`self.TL_HitBraum`) (/ 1.0 0.25))
      (bind (_direction_2 _alpha_2) (`Timeline|TL_HitBraum` :!via `PlayFromStart`)
        (:`Update`
          (`self.K2_SetActorLocation` self (`KismetMathLibrary.VLerp` (`self.EndLocAttackBraum`) (`self.StartLocAttackBraum`) _alpha_2) false false))
        (:`Finished`
          (if (< (`KismetMathLibrary.Vector_Distance` (`self.K2_GetActorLocation` self) (`self.K2_GetActorLocation` (`self.Player`))) 550.0)
            (`KismetSystemLibrary.PrintString` "Hit")
            (else
              (`KismetSystemLibrary.PrintString` "Miss")))
          (set `CharacterMovementComponent.GravityScale` 1.0 (`self.CharacterMovement`))
          (set `self.Braum ATK` true)
          (`/Game/Blueprints/Character/BP_Character.takedamage` (`self.Player`) (`KismetMathLibrary.Conv_IntToDouble` (`KismetMathLibrary.RandomIntegerInRange` 10 15)))
          (`self.Braum_StartPatrol`))))))

(event `DistanceSetup`
  (bind _mesh (`self.Mesh`))
  ;[0 0 1 0.1] Distance
  (bind _returnvalue (`KismetSystemLibrary.K2_SetTimerDelegate` (delegate `CodeDistance`) 0.25 true))
  (set `self.HandleTimerDistanceBase` _returnvalue)
  (bind _output_get (set `self.MaxHealth` 75.0))
  (set `self.CurrentHealth` _output_get)
  (set `CharacterMovementComponent.MaxWalkSpeed` 700.0 (`self.CharacterMovement`))
  (`SkeletalMeshComponent.SetSkeletalMeshAsset` _mesh "/Game/Blueprints/Ennemi/mesh/Tireuse/tireuse__2_.tireuse__2_")
  (`SkeletalMeshComponent.PlayAnimation` _mesh "/Game/Blueprints/Ennemi/mesh/Tireuse/anim/BS_tireuse.BS_tireuse" true)
  (`self.PatrolDistance`)
  (`/Engine/EditorBlueprintResources/StandardMacros.DoOnce` false
    (:`Completed`
      (bind _returnvalue_2 (`GameplayStatics.GetActorOfClass` "/Game/Blueprints/Manager/BP_GameManager.BP_GameManager_C"))
      (set `self.GameManager` _returnvalue_2))))

(event `PatrolDistance`
  ;[0 0 1 0.1] Distance
  (bind _returnvalue (`KismetSystemLibrary.K2_SetTimerDelegate` (delegate `CodeDistancePatrol`) 0.25 true))
  (set `self.HandleTimerDistance` _returnvalue))

(event `CodeDistance`
  ;[0 0 1 0.1] Distance
  (if (not (> (`KismetMathLibrary.Vector_Distance` (`self.K2_GetActorLocation` (`self.Player`)) (`self.K2_GetActorLocation` self)) 1000.0))
    (`/Engine/EditorBlueprintResources/StandardMacros.DoOnce` false :!label _label_3
      (:`Completed`
        (`self.AttackDistance`)))))

(event `ResetDoOnceDistance`
  ;[0 0 1 0.1] Distance
  (goto _label_3 :!via `Reset`))

(event `CodeDistancePatrol`
  (bind (_returnvalue_roll _returnvalue_pitch _returnvalue_yaw) (`KismetMathLibrary.BreakRotator` (`KismetMathLibrary.FindLookAtRotation` (`self.K2_GetActorLocation` self) (`self.K2_GetActorLocation` (`self.Player`)))))
  ;[0 0 1 0.1] Distance
  (`|AIMoveTo` self (0.0 0.0 0.0) (`self.Player`)
    (:`then`
      (`TimelineComponent.SetPlayRate` (`self.TL_DistancePatrol`) (/ 1.0 0.24))
      (`Timeline|TL_DistancePatrol` :!via `PlayFromStart`
        (:`Update`
          (`self.K2_SetActorRotation` self (`KismetMathLibrary.MakeRotator` 0.0 0.0 _returnvalue_yaw) false))))))

(event `AttackDistance`
  (bind _player (`self.Player`))
  ;[0 0 1 0.1] Distance
  (`KismetSystemLibrary.K2_ClearAndInvalidateTimerHandle` (`self.HandleTimerDistance`))
  (`MovementComponent.StopMovementImmediately` (`self.CharacterMovement`))
  (set `self.SpawnBulletLocation` (`SceneComponent.K2_GetComponentLocation` (`self.SpawnLocation`)))
  (bind _returnvalue (`|SpawnActorFromClass` "/Game/Blueprints/Ennemi/BP_ThrowableObject.BP_ThrowableObject_C" (`KismetMathLibrary.MakeTransform` (`self.SpawnBulletLocation`)) "AdjustIfPossibleButAlwaysSpawn" "MultiplyWithRoot" null null))
  (set `self.CurrentBullet` _returnvalue)
  (`KismetArrayLibrary.Array_Clear` (`self.PointsThrowDirection`))
  (`KismetArrayLibrary.Array_Add` (`self.PointsThrowDirection`) (`self.SpawnBulletLocation`))
  (set `self.EndBulletLocation` (- (`self.K2_GetActorLocation` (`self.Player`)) (0.0 0.0 80.0)))
  (`KismetArrayLibrary.Array_Add` (`self.PointsThrowDirection`) (`self.EndBulletLocation`))
  (`KismetArrayLibrary.Array_Insert` (`self.PointsThrowDirection`) (+ (/ (+ (`self.SpawnBulletLocation`) (`self.EndBulletLocation`)) 2.0) (0.0 0.0 500.0)) 1)
  (`SplineComponent.SetSplinePoints` (`/Game/Blueprints/Manager/BP_GameManager.SplineThrowDistance` (`self.GameManager`)) (`self.PointsThrowDirection`) "World" true)
  (`TimelineComponent.SetPlayRate` (`self.TL_Throw`) (/ 1.0 (`self.ThrowDuration`)))
  (bind (_direction _alpha) (`Timeline|TL_Throw` :!via `PlayFromStart`)
    (:`Update`
      (`self.K2_SetActorLocation` (`self.CurrentBullet`) (`SplineComponent.GetLocationAtTime` (`/Game/Blueprints/Manager/BP_GameManager.SplineThrowDistance` (`self.GameManager`)) _alpha "World" false) false false))
    (:`Finished`
      (set `self.dist atk` true)
      (`/Game/Blueprints/Character/BP_Character.takedamage` _player (`KismetMathLibrary.Conv_IntToDouble` (`KismetMathLibrary.RandomIntegerInRange` 2 5)))
      (`KismetSystemLibrary.PrintString` (`KismetStringLibrary.Conv_DoubleToString` (`/Game/Blueprints/Character/BP_Character.current health` _player)))
      (`self.DistanceSetup`)
      (`self.ResetDoOnceDistance`)
      (`KismetSystemLibrary.Delay` 0.2)
      (`self.K2_DestroyActor` (`self.CurrentBullet`)))))

(event `ClearAllTimer`
  ; Clear Timer
  (`KismetSystemLibrary.K2_ClearAndInvalidateTimerHandle` (`self.Handle_Patrol`))
  (`KismetSystemLibrary.K2_ClearAndInvalidateTimerHandle` (`self.Handle_Patrol_Braum`))
  (`KismetSystemLibrary.K2_ClearAndInvalidateTimerHandle` (`self.HandleTimerDistance`))
  (`MovementComponent.StopMovementImmediately` (`self.CharacterMovement`))
  (`self.OnSwitch`))

(event `takedamageE`
  (params (damage :type "Float (double-precision)"))
  ; Take Damage
  (bind _output_get (set `self.CurrentHealth` (- (`self.CurrentHealth`) damage)))
  (if (<= _output_get 0.0)
    (`/Game/UI/WB_Score.UpdateCombo` (`/Game/Blueprints/Manager/BP_GameManager.WB_Score` (`self.GameManager`)))
    (if (`KismetSystemLibrary.IsValid` (`self.CurrentBullet`))
      (`self.K2_DestroyActor` (`self.CurrentBullet`))
      (`self.K2_DestroyActor`)
      (else
        (`self.K2_DestroyActor`)))))

(fn `UserConstructionScript`)