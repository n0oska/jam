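; BP_flaque is a temporary puddle hazard that slows characters standing in it and destroys itself five seconds after spawning.
; Its Box overlap events halve the CharacterMovement MaxWalkSpeed of any BP_EnnemiParent or BP_Character on entry and double it on exit.
; The change is relative to the current speed, with no stored original value.
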(event `self.ReceiveBeginPlay`
  (`KismetSystemLibrary.Delay` 5.0)
  (`self.K2_DestroyActor`))

(event `self.Box.OnComponentBeginOverlap`
  (params (OverlappedComponent :type "PrimitiveComponent Object Reference") (OtherActor :type "Actor Object Reference") (OtherComp :type "PrimitiveComponent Object Reference") (OtherBodyIndex :type Integer) (bFromSweep :type Boolean) (SweepResult :type "HitResult Structure (by ref)"))
  (bind (_asbp_ennemi_parent _bsuccess) (cast `/Game/Blueprints/Ennemi/BP_EnnemiParent` OtherActor :!pure true))
  (bind (_asbp_character _bsuccess_2) (cast `/Game/Blueprints/Character/BP_Character` OtherActor :!pure true))
  (bind _charactermovement (`Character.CharacterMovement` _asbp_character))
  (bind _charactermovement_2 (`Character.CharacterMovement` _asbp_ennemi_parent))
  (if _bsuccess
    (set `CharacterMovementComponent.MaxWalkSpeed` (/ (`CharacterMovementComponent.MaxWalkSpeed` _charactermovement_2) 2.0) _charactermovement_2)
    (elif _bsuccess_2
      (set `CharacterMovementComponent.MaxWalkSpeed` (/ (`CharacterMovementComponent.MaxWalkSpeed` _charactermovement) 2.0) _charactermovement))))

(event `self.Box.OnComponentEndOverlap`
  (params (OverlappedComponent :type "PrimitiveComponent Object Reference") (OtherActor :type "Actor Object Reference") (OtherComp :type "PrimitiveComponent Object Reference") (OtherBodyIndex :type Integer))
  (bind (_asbp_ennemi_parent _bsuccess) (cast `/Game/Blueprints/Ennemi/BP_EnnemiParent` OtherActor :!pure true))
  (bind (_asbp_character _bsuccess_2) (cast `/Game/Blueprints/Character/BP_Character` OtherActor :!pure true))
  (bind _charactermovement (`Character.CharacterMovement` _asbp_character))
  (bind _charactermovement_2 (`Character.CharacterMovement` _asbp_ennemi_parent))
  (if _bsuccess
    (set `CharacterMovementComponent.MaxWalkSpeed` (* (`CharacterMovementComponent.MaxWalkSpeed` _charactermovement_2) 2.0) _charactermovement_2)
    (elif _bsuccess_2
      (set `CharacterMovementComponent.MaxWalkSpeed` (* (`CharacterMovementComponent.MaxWalkSpeed` _charactermovement) 2.0) _charactermovement))))

(fn `UserConstructionScript`)