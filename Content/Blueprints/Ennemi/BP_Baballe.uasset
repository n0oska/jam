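; BP_Baballe is an enemy hazard actor that descends from its spawn point, sprays bullet balls, then destroys itself.
; On BeginPlay a timeline lowers it 500 units over its descent.
; When that finishes, a looping timer rapidly spawns BP_BulletBaballe at the end point with random rotation, physics and collision disabled, while a second timeline shrinks its sphere to zero.
; The timer clears and the actor is destroyed after about four seconds.
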(event `self.ReceiveBeginPlay`
  (`self.SetupSpawn`)
  (set `self.Timer` 0.0))

(event `SetupSpawn`
  (bind _returnvalue (`self.K2_GetActorLocation` self))
  (set `self.StartLocation` _returnvalue)
  (set `self.EndLocation` (- _returnvalue (0.0 0.0 500.0)))
  (`TimelineComponent.SetPlayRate` (`self.TL_GoLow`) (/ 1.0 4.0))
  (bind (_direction _alpha) (`Timeline|TL_GoLow` :!via `PlayFromStart`)
    (:`Update`
      (`self.K2_SetActorLocation` (`KismetMathLibrary.VLerp` (`self.StartLocation`) (`self.EndLocation`) _alpha)))
    (:`Finished`
      (`self.TimerSpawnBall`)
      (set `self.BaseScale` (`SceneComponent.K2_GetComponentScale` (`self.Sphere`)))
      (`TimelineComponent.SetPlayRate` (`self.TL_ScaleDown`) (/ 1.0 4.0))
      (bind (_direction_2 _alpha_2) (`Timeline|TL_ScaleDown` :!via `PlayFromStart`)
        (:`Update`
          (`SceneComponent.SetWorldScale3D` (`self.Sphere`) (`KismetMathLibrary.VLerp` (`self.BaseScale`) (0.0 0.0 0.0) _alpha_2)))))))

(event `TimerSpawnBall`
  (bind _returnvalue (`KismetSystemLibrary.K2_SetTimerDelegate` (delegate `Code`) 0.05 true)))

(event `Code`
  (bind _returnvalue (`|SpawnActorFromClass` "/Game/Blueprints/Ennemi/BP_BulletBaballe.BP_BulletBaballe_C" (`KismetMathLibrary.MakeTransform` (`self.EndLocation`) (`KismetMathLibrary.RandomRotator` false)) "AdjustIfPossibleButAlwaysSpawn" "MultiplyWithRoot" null null))
  (bind _sphere (`/Game/Blueprints/Ennemi/BP_BulletBaballe.Sphere` _returnvalue))
  (`PrimitiveComponent.SetSimulatePhysics` _sphere false)
  (`PrimitiveComponent.SetCollisionEnabled` _sphere "NoCollision")
  (bind _output_get (set `self.Timer` (+ (`self.Timer`) 0.05)))
  (if (> _output_get 4.0)
    (`KismetSystemLibrary.K2_ClearAndInvalidateTimerHandle` (stale `TimerSpawnBall` _returnvalue))
    (`self.K2_DestroyActor`)))

(fn `UserConstructionScript`)