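; BP_BulletBaballe is an enemy bullet that bounces once and leaves a puddle.
; On BeginPlay its Sphere has collision and physics off, then enables both after a one-second delay.
; The first Sphere hit only sets the Compteur flag; the next hit destroys the actor and spawns BP_flaque at the impact location.
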(event `self.ReceiveBeginPlay`
  (bind _sphere (`self.Sphere`))
  (bind _sphere_2 (`self.Sphere`))
  (`PrimitiveComponent.SetCollisionEnabled` _sphere "NoCollision")
  (`PrimitiveComponent.SetSimulatePhysics` _sphere false)
  (`KismetSystemLibrary.Delay` 1.0)
  (`PrimitiveComponent.SetCollisionEnabled` _sphere_2 "QueryAndPhysics")
  (`PrimitiveComponent.SetSimulatePhysics` _sphere_2 true))

(event `self.Sphere.OnComponentHit`
  (params (HitComponent :type "PrimitiveComponent Object Reference") (OtherActor :type "Actor Object Reference") (OtherComp :type "PrimitiveComponent Object Reference") (NormalImpulse :type "Vector Structure") (Hit :type "HitResult Structure (by ref)"))
  (if (`self.Compteur`)
    (`|ExecutionSequence`
      (:`then_0`
        (`self.K2_DestroyActor`))
      (:`then_1`
        (`|SpawnActorFromClass` "/Game/Blueprints/Ennemi/BP_flaque.BP_flaque_C" (`KismetMathLibrary.MakeTransform` Hit_Location) "AdjustIfPossibleButAlwaysSpawn" "MultiplyWithRoot" null null)))
    (else
      (set `self.Compteur` true))))

(fn `UserConstructionScript`)