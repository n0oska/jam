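; Game manager that runs the score HUD and triggers arena events that change gameplay during play.
; BeginPlay creates the score widget, caches player and spawner, then starts a looping 30-second timer.
; Nested FlipFlops rotate its events: one-time pillar sequence plus ball spawn, spawner and player enemy-type change, temporary bouncy surfaces, random retyping of live enemies.
; Timelines animate score counting and chain each random pillar's rise and return until none remain.
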(event `self.ReceiveBeginPlay`
  (bind _returnvalue (`|CreateWidget` "/Game/UI/WB_Score.WB_Score_C"))
  (bind _output_get (set `self.WB_Score` _returnvalue))
  (`UserWidget.AddToViewport` _output_get 0)
  (bind _returnvalue_2 (`GameplayStatics.GetActorOfClass` "/Game/Blueprints/Character/BP_Character.BP_Character_C"))
  (set `self.Player` _returnvalue_2)
  (bind _returnvalue_3 (`GameplayStatics.GetActorOfClass` "/Game/Blueprints/Manager/BP_SpawnerManager.BP_SpawnerManager_C"))
  (set `self.SpawnerManager` _returnvalue_3)
  (`self.TimerEvent`))

(event `UpdateScore`
  (params (Score :type "Float (double-precision)"))
  ;[1 0 0 0.1] Score
  (set `self.NewScore` Score)
  (`TimelineComponent.SetPlayRate` (`self.TL_UpdateScore`) (/ 1.0 0.75))
  (bind (_direction _alpha) (`Timeline|TL_UpdateScore` :!via `PlayFromStart`)
    (:`Update`
      (`RichTextBlock.SetText` (`/Game/UI/WB_Score.Score` (`self.WB_Score`)) (`|FormatText` "<Score>Score : {Score}</>" (`KismetMathLibrary.Lerp` (`self.CurrentScore`) (`self.NewScore`) _alpha))))
    (:`Finished`
      (set `self.CurrentScore` (`self.NewScore`)))))

(event `Basic`
  (bind _player (`self.Player`))
  (set `/Game/Blueprints/Manager/BP_SpawnerManager.EnnemiType` 0 (`self.SpawnerManager`))
  (set `/Game/Blueprints/Character/BP_Character.enemytype` 0 _player)
  (`/Game/Blueprints/Character/BP_Character.SwitchEnnemi` _player))

(event `Braum`
  (bind _player (`self.Player`))
  (set `/Game/Blueprints/Manager/BP_SpawnerManager.EnnemiType` 1 (`self.SpawnerManager`))
  (set `/Game/Blueprints/Character/BP_Character.enemytype` 1 _player)
  (`/Game/Blueprints/Character/BP_Character.SwitchEnnemi` _player))

(event `Distance`
  (bind _player (`self.Player`))
  (set `/Game/Blueprints/Manager/BP_SpawnerManager.EnnemiType` 2 (`self.SpawnerManager`))
  (set `/Game/Blueprints/Character/BP_Character.enemytype` 2 _player)
  (`/Game/Blueprints/Character/BP_Character.SwitchEnnemi` _player))

(event `TimerSwitchEnnemy/Weapons`
  (switch `int` (`/Game/Blueprints/Manager/BP_SpawnerManager.EnnemiType` (`self.SpawnerManager`))
    (:`0`
      (`self.Basic`))
    (:`1`
      (`self.Braum`))
    (:`2`
      (`self.Distance`))))

(event `TimerEvent`
  (`KismetSystemLibrary.K2_SetTimerDelegate` (delegate `CodeEvent`) 30.0 true))

(event `CodeEvent`
  (`/Engine/EditorBlueprintResources/StandardMacros.FlipFlop`
    (:`A`
      (`/Engine/EditorBlueprintResources/StandardMacros.FlipFlop`
        (:`A`
          (`/Engine/EditorBlueprintResources/StandardMacros.DoOnce` false
            (:`Completed`
              (`self.Pillar`)
              (`self.EventBalle`))))
        (:`B`
          (`self.EventBounciness`))))
    (:`B`
      (`/Engine/EditorBlueprintResources/StandardMacros.FlipFlop`
        (:`A`
          (`self.GoDistance`))
        (:`B`
          (`self.EventSwitchEnnemy`))))))

(event `EventBalle`
  (`|SpawnActorFromClass` "/Game/Blueprints/Ennemi/BP_Baballe.BP_Baballe_C" (`KismetMathLibrary.MakeTransform` (0.0 0.0 15000.0)) "AdjustIfPossibleButAlwaysSpawn" "MultiplyWithRoot" null null))

(event `EventSwitchEnnemy`
  ; PAS OUBLIER NIAGARA SYSTEM DE FUMEE
  (bind _outactors (`GameplayStatics.GetAllActorsOfClass` "/Game/Blueprints/Ennemi/BP_EnnemiParent.BP_EnnemiParent_C"))
  (for _array_element _outactors
    (set `/Game/Blueprints/Ennemi/BP_EnnemiParent.EnnemiType` (`KismetArrayLibrary.Array_Random` (`self.AllEnnemyType`)) _array_element)
    (`/Game/Blueprints/Ennemi/BP_EnnemiParent.ClearAllTimer` _array_element)))

(event `GoDistance`
  (`/Game/Blueprints/Manager/BP_SpawnerManager.UpdateSpawner` (`self.SpawnerManager`) 1)
  (set `/Game/Blueprints/Character/BP_Character.enemytype` 1 (`self.Player`))
  (`/Game/Blueprints/Character/BP_Character.SwitchEnnemi` (`self.Player`)))

(event `EventBounciness`
  (bind _outactors (`GameplayStatics.GetAllActorsOfClass` "/Game/Blueprints/Enviro/BP_Bounciness.BP_Bounciness_C"))
  (bind _output_get (set `self.AllBounci` _outactors))
  (for _array_element _output_get
    (set `/Game/Blueprints/Enviro/BP_Bounciness.bCanBounce` true _array_element))
  (set `/Game/Blueprints/Manager/BP_SpawnerManager.EnnemiType` 2 (`self.SpawnerManager`))
  (`KismetSystemLibrary.Delay` 30.0)
  (`self.StopBounciness`))

(event `StopBounciness`
  (for _array_element (`self.AllBounci`)
    (set `/Game/Blueprints/Enviro/BP_Bounciness.bCanBounce` false _array_element)))

(event `Pillar`
  (bind _outitem (`KismetArrayLibrary.Array_Random` (`self.AllPilars`)))
  (if (`KismetSystemLibrary.IsValid` _outitem)
    (bind _output_get (set `self.CurrentPillar` _outitem))
    (`StaticMeshActor.SetMobility` _output_get "Movable")
    (bind _returnvalue (`self.K2_GetActorLocation` _output_get))
    (set `self.CurrentBaseLoc` _returnvalue)
    (set `self.CurrentEndLoc` (+ _returnvalue (0.0 0.0 700.0)))
    (`TimelineComponent.SetPlayRate` (`self.TL_Pillars`) (/ 1.0 5.0))
    (bind (_direction _alpha) (`Timeline|TL_Pillars` :!via `PlayFromStart`)
      (:`Update`
        (`self.K2_SetActorLocation` (`self.CurrentPillar`) (`KismetMathLibrary.VLerp` (`self.CurrentBaseLoc`) (`self.CurrentEndLoc`) _alpha) false false))
      (:`Finished`
        (`KismetArrayLibrary.Array_RemoveItem` (`self.AllPilars`) (`self.CurrentPillar`))
        (`TimelineComponent.SetPlayRate` (`self.TL_PillarGoBack`) (/ 1.0 3.0))
        (bind (_direction_2 _alpha_2) (`Timeline|TL_PillarGoBack` :!via `PlayFromStart`)
          (:`Update`
            (`self.K2_SetActorLocation` (`self.CurrentPillar`) (`KismetMathLibrary.VLerp` (`self.CurrentEndLoc`) (`self.CurrentBaseLoc`) _alpha_2) false false))
          (:`Finished`
            (`self.Pillar`)))))))

(fn `F_Balle`
  (`self.EventBalle`))

(fn `F_SwitchEnnemi`
  (`self.EventSwitchEnnemy`))

(fn `UserConstructionScript`)