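; BP_SpawnerManager is a manager that periodically randomizes which enemy type each spawner in the level is set to spawn.
; On BeginPlay it caches all BP_Spanwer actors and starts a looping 30-second timer.
; Each tick of that timer independently assigns every cached spawner a random entry from AllEnnemiType, using a hard-coded index range covering the first three entries.
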(event `self.ReceiveBeginPlay`
  (bind _outactors (`GameplayStatics.GetAllActorsOfClass` "/Game/Blueprints/Ennemi/BP_Spanwer.BP_Spanwer_C"))
  (set `self.AllSpaawner` _outactors)
  (`self.StartSpawner`))

(event `StartSpawner`
  (`KismetSystemLibrary.K2_SetTimerDelegate` (delegate `Code`) 30.0 true))

(event `Code`
  (for _array_element (`self.AllSpaawner`)
    (set `/Game/Blueprints/Ennemi/BP_Spanwer.EnnemiTypeToSpawn` (`|GetArrayItem` (`self.AllEnnemiType`) (`KismetMathLibrary.RandomIntegerInRange` 0 2)) _array_element)))

(fn `UserConstructionScript`)